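; BP_Checpoint is a race checkpoint that records car progress and moves the respawn point of each BP_Base_car that passes through it.
; When a car overlaps its Box, it adds the car with this checkpoint's Id to the QuiPasse map on the first BP_Depart found in the level.
; It then sets the car's respawn position to the checkpoint's location and its respawn rotation to the Arrow's world rotation.
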(event `self.Box.OnComponentBeginOverlap`
  (params (OverlappedComponent :type "PrimitiveComponent Object Reference") (OtherActor :type "Actor Object Reference") (OtherComp :type "PrimitiveComponent Object Reference") (OtherBodyIndex :type Integer) (bFromSweep :type Boolean) (SweepResult :type "HitResult Structure (by ref)"))
  (bind _asbp_base_car (cast `/Game/Car/BP_Base_car` OtherActor))
  (bind _outactors (`GameplayStatics.GetAllActorsOfClass` "/Game/BP/BP_Depart.BP_Depart_C"))
  (`BlueprintMapLibrary.Map_Add` (`/Game/BP/BP_Depart.quiPasse` (`|GetArrayItem` _outactors)) _asbp_base_car (`checkpoint_id_prop.id` (`self.checkpoint_id_prop`)))
  (set `/Game/Car/BP_Base_car.respawn_pos` (`self.K2_GetActorLocation`) _asbp_base_car)
  (set `/Game/Car/BP_Base_car.respawn_rot` (`SceneComponent.K2_GetComponentRotation` (`self.Arrow`)) _asbp_base_car))

(fn `UserConstructionScript`)