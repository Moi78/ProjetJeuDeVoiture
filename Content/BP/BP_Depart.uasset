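; Start line trigger ("Depart") that counts laps for each actor crossing it, apparently for a race.
; On box overlap it turns two meshes green, sets EstPasse and records StartTime in real-time hundredths of a second.
; Actors already in the QuiPasse map get their entry reset to zero, their Lap count incremented and debug prints.
; New actors are added to QuiPasse, but their Lap add has no key connected.
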(event `self.Box.OnComponentBeginOverlap`
  (params (OverlappedComponent :type "PrimitiveComponent Object Reference") (OtherActor :type "Actor Object Reference") (OtherComp :type "PrimitiveComponent Object Reference") (OtherBodyIndex :type Integer) (bFromSweep :type Boolean) (SweepResult :type "HitResult Structure (by ref)"))
  (bind _quipasse (`self.quiPasse`))
  (bind _lap (`self.lap`))
  (`MeshComponent.SetVectorParameterValueOnMaterials` (`self.StaticMesh1`) "Color" (0.0 255.0 0.0))
  (`MeshComponent.SetVectorParameterValueOnMaterials` (`self.StaticMesh`) "Color" (0.0 255.0 0.0))
  (set `self.estPasse` true)
  ;[1 1 1] Check si le joueur est déjà passé
  (set `self.startTime` (`KismetMathLibrary.FTrunc` (* (`GameplayStatics.GetRealTimeSeconds`) 100.0)))
  (if (`.ReturnValue` (`BlueprintMapLibrary.Map_Find` (`self.quiPasse`) OtherActor))
    (`BlueprintMapLibrary.Map_Add` _quipasse OtherActor)
    (`BlueprintMapLibrary.Map_Add` _lap OtherActor (+ (`BlueprintMapLibrary.Map_Find` _lap OtherActor) 1))
    ;[1 1 1] Debug
    (bind _keys (`BlueprintMapLibrary.Map_Keys` _quipasse))
    (for _array_element _keys
      (`KismetSystemLibrary.PrintString` (`KismetStringLibrary.Conv_IntToString` (`BlueprintMapLibrary.Map_Find` (`self.quiPasse`) _array_element)))
      (`KismetSystemLibrary.PrintString` (`KismetSystemLibrary.GetDisplayName` _array_element)))
    (else
      (`BlueprintMapLibrary.Map_Add` _quipasse OtherActor)
      (`BlueprintMapLibrary.Map_Add` _lap))))

(fn `UserConstructionScript`)