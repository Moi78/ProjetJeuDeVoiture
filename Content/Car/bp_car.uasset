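; Drivable car Blueprint that can respawn at the start point when R is pressed.
; Movement axes feed throttle and steering into VehicleMovement, while mouse axes turn the controller for a debug spring-arm camera.
; BeginPlay caches the arrow transform of the first BP_Depart found as the respawn point.
; Teleport stops all movement before moving the car there; both authority and remote branches call it.
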(event `Key|R`
  (params (Key :type "Key Structure"))
  ;[1 1 1] Respawn
  (:`Pressed`
    (`/Engine/EditorBlueprintResources/ActorMacros.Switch Has Authority`
      (:`Authority`
        (`self.Teleport`))
      (:`Remote`
        (`self.Teleport`)))))

(event `Teleport`
  ;[1 1 1] Respawn
  (`bpCustomNode.StopEveryMovement` (`self.Mesh`) (`self.VehicleMovement`))
  (`self.K2_SetActorTransform` (`KismetMathLibrary.MakeTransform` (`self.Respawn_Pos`) (`self.Respawn_Rot`)) false true))

(event `InputAxisKey|MouseX`
  (params (AxisValue :type "Float (single-precision)"))
  ;[1 1 1] Debug (Rotation du spring arm en fonction du mvt de la souris)
  (`self.AddControllerYawInput` AxisValue))

(event `InputAxis|move_forward`
  (params (AxisValue :type "Float (single-precision)"))
  ;[1 1 1] Mouvement
  (`WheeledVehicleMovementComponent.SetThrottleInput` (`self.VehicleMovement`) AxisValue))

(event `InputAxisKey|MouseY`
  (params (AxisValue :type "Float (single-precision)"))
  ;[1 1 1] Debug (Rotation du spring arm en fonction du mvt de la souris)
  (`self.AddControllerPitchInput` (* AxisValue -1.0)))

(event `InputAxis|move_right`
  (params (AxisValue :type "Float (single-precision)"))
  ;[1 1 1] Mouvement
  (`WheeledVehicleMovementComponent.SetSteeringInput` (`self.VehicleMovement`) AxisValue))

(event `self.ReceiveBeginPlay`
  ;[1 1 1] Initialisation respawn
  (bind _outactors (`GameplayStatics.GetAllActorsOfClass` "/Game/BP/BP_Depart.BP_Depart_C"))
  (bind _arrow (`/Game/BP/BP_Depart.Arrow` (`|GetArrayItem` _outactors)))
  (set `self.Respawn_Pos` (`SceneComponent.K2_GetComponentLocation` _arrow))
  (set `self.Respawn_Rot` (`SceneComponent.K2_GetComponentRotation` _arrow)))

(fn `UserConstructionScript`)